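; Automated turret building that detects nearby objects with a sphere trace every Tick and shoots at them.
; An Idle/OnBattle state starts a looping Fire timer on detection, which spawns Bullet_BP with random pitch and roll spread.
; In battle, BarrelRotate eases the barrel toward the hit point, or toward zero rotation when nothing is detected.
; The timer stops only once the barrel rotation reaches near zero.
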(event `self.ReceiveBeginPlay`)

(event `self.ReceiveTick`
  (params (DeltaSeconds :type "Float (single-precision)"))
  (bind _returnvalue (`self.K2_GetActorLocation`))
  (bind (_outhit _returnvalue_2) (`KismetSystemLibrary.SphereTraceSingleForObjects` :`Start` _returnvalue :`End` _returnvalue :`Radius` 5000.0 :`ObjectTypes` (`|MakeArray` "ObjectTypeQuery7" :!type "EObjectTypeQuery Enum") :`DrawDebugType` "ForOneFrame"))
  (switch `/Game/Buildings/Weapon/Turret_State` (`self.IsInBattle`)
    (:`NewEnumerator0`
      (if _returnvalue_2
        (`self.AttackOn`)))
    (:`NewEnumerator1`
      (bind _on_origin (`self.Barrel Rotate` (`.ImpactPoint` (`GameplayStatics.BreakHitResult` _outhit)) _returnvalue_2))
      (if _on_origin
        (`self.AttackOff`)))))

(fn `AttackOff`
  (`KismetSystemLibrary.K2_ClearAndInvalidateTimerHandle` (`self.AttackTimer`))
  (set `self.IsInBattle` "NewEnumerator0"))

(fn `AttackOn`
  (set `self.IsInBattle` "NewEnumerator1")
  (bind _returnvalue (`KismetSystemLibrary.K2_SetTimer` null "Fire" (`self.FireRate`) true))
  (set `self.AttackTimer` _returnvalue))

(fn `Barrel Rotate`
  (params (`Target Loc` :type "Vector Structure") (`To Target` :type Boolean))
  (returns (`On Origin` :type Boolean))
  (bind _turret_barrel_point (`self.Turret Barrel Point`))
  (bind _returnvalue (`KismetMathLibrary.RInterpTo` (`SceneComponent.K2_GetComponentRotation` _turret_barrel_point) (`KismetMathLibrary.SelectRotator` (`KismetMathLibrary.FindLookAtRotation` (`self.K2_GetActorLocation`) `Target Loc`) (struct) `To Target`) 0.1 2.0))
  (bind _returnvalue_2 (== _returnvalue (struct) :`ErrorTolerance` 0.1))
  (`SceneComponent.K2_SetWorldRotation` _turret_barrel_point _returnvalue false false)
  (if _returnvalue_2
    (`SceneComponent.K2_SetWorldRotation` :`self` _turret_barrel_point)
    (return _returnvalue_2)
    (else
      (return false))))

(fn `Fire`
  (bind _shoot (`self.Shoot`))
  (bind (_relativerotation_roll _relativerotation_pitch _relativerotation_yaw) (`KismetMathLibrary.BreakRotator` (`SceneComponent.RelativeRotation` _shoot)))
  (`SceneComponent.K2_SetRelativeRotation` _shoot (`KismetMathLibrary.MakeRotator` (`KismetMathLibrary.RandomFloatInRange` -5.0 5.0) (`KismetMathLibrary.RandomFloatInRange` -5.0 5.0) _relativerotation_yaw) false false)
  (`|SpawnActorFromClass` "/Game/Buildings/Weapon/Bullet_BP.Bullet_BP_C" (`SceneComponent.K2_GetComponentToWorld` _shoot) "Undefined" "MultiplyWithRoot" null 5000.0 7.0 null))

(fn `UserConstructionScript`)